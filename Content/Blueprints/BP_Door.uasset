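; BP_Door is a door actor that slides vertically when driven by a BP_Button.
; On BeginPlay it finds a BP_Button with GetActorOfClass and binds its OPEN and CLOSE events to that button's open and close events.
; OPEN and CLOSE use MoveComponentTo to shift the static mesh up or down by a fixed offset, passing its current world location plus the offset as the relative target.
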(event `self.ReceiveBeginPlay`
  (bind _returnvalue (`GameplayStatics.GetActorOfClass` "/Game/Blueprints/BP_Button.BP_Button_C"))
  (bind _output_get (set `self.Button Ref` _returnvalue))
  (add `/Game/Blueprints/BP_Button.Open` _output_get (delegate `OPEN`))
  (add `/Game/Blueprints/BP_Button.Close` _output_get (delegate `CLOSE`)))

(event `OPEN`
  (bind _staticmeshcomponent (`self.StaticMeshComponent`))
  (`KismetSystemLibrary.MoveComponentTo` _staticmeshcomponent (+ (`SceneComponent.K2_GetComponentLocation` _staticmeshcomponent) (0.0 0.0 500.0))))

(event `CLOSE`
  (bind _staticmeshcomponent (`self.StaticMeshComponent`))
  (`KismetSystemLibrary.MoveComponentTo` _staticmeshcomponent (- (`SceneComponent.K2_GetComponentLocation` _staticmeshcomponent) (0.0 0.0 500.0))))

(fn `UserConstructionScript`)